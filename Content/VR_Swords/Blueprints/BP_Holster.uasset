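; BP_Holster is a VR sword holster that serves either as a body holster on MotionControllerPawnSwords or as a fixed mount.
; The construction script casts the parent actor to choose belt and back or mount meshes and collision, then applies custom meshes and optional transparency.
; When attached, Tick places it below the camera with a height offset, following yaw only, blending forward toward up vector when looking down to keep heading stable.
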(event EventTick
  (params (DeltaSeconds :type Float%20%28single-precision%29))
  (bind _parentreference (Variables|Default|GetParentReference))
  (bind _defaultsceneroot (Variables|Default|GetDefaultSceneRoot))
  (bind _camera (Variables|/Game/VR_Swords/Pawn/MotionControllerPawnSwords.MotionControllerPawnSwords_C|GetCamera _parentreference))
  (bind _returnvalue (Math|Vector|GetForwardVector _camera))
  (bind _returnvalue_2 (Math|Vector|GetUpVector _camera))
  (bind _returnvalue_3 (Transformation|GetWorldLocation _camera))
  (bind _returnvalue_4 (* _returnvalue_2 -11.0))
  (bind _returnvalue_5 (+ _returnvalue_3 _returnvalue_4))
  (bind (_x _y _z) (Math|Vector|BreakVector _returnvalue_5))
  ;[1 1 1] This checks the location of the player's head, and sets the location of the holster accordingly
  (if (Variables|Default|GetIsAttachedToPawn)
    (Transformation|SetWorldLocation _defaultsceneroot (Math|Vector|MakeVector _x _y (- _z (Variables|Default|GetHeightOffset))) false false)
    (Transformation|SetWorldRotation _defaultsceneroot (Math|Rotator|MakeRotator 0.0 0.0 (.Yaw (Math|Rotator|BreakRotator (Math|Conversions|RotationFromXVector (Math|Vector|Lerp(Vector) _returnvalue (Math|Vector|GetUpVector _camera) (Math|Float|Absolute(Float) (Math|Float|Clamp(Float) (.Z (Math|Vector|BreakVector _returnvalue)) -1.0 0.0))))))) false false)))

(fn ConstructionScript
  (bind _fixedmount (Variables|Default|GetFixedMount))
  (bind _holsterback (Variables|Default|GetHolsterBack))
  (bind _custombeltmesh (Variables|Default|GetCustomBeltMesh))
  (bind _custombackmesh (Variables|Default|GetCustomBackMesh))
  (bind _customfixedmesh (Variables|Default|GetCustomFixedMesh))
  ;[1 1 1] This sets the ParentReference to the MotionControllerPawn. If you use a Custom Pawn, change the Cast to Node to cast to your pawn, and also change the Variable Type of ParentReference to match your Pawn
  (bind _asmotion_controller_pawn_swords (Utilities|Casting|CastToMotionControllerPawnSwords (Actor|GetParentActor))
    (:then
      (Variables|Default|SetParentReference _asmotion_controller_pawn_swords)
      (Collision|SetCollisionEnabled _fixedmount "NoCollision")
      (Rendering|SetVisibility _fixedmount false false)
      (Collision|SetCollisionEnabled _holsterback "QueryOnly")
      (Rendering|SetVisibility _holsterback true false)
      (Variables|Default|SetIsAttachedToPawn true)
      (Utilities|Array|Clear (Variables|Actor|GetTags)))
    (:CastFailed
      (Collision|SetCollisionEnabled _fixedmount "QueryOnly")
      (Rendering|SetVisibility _fixedmount true false)
      (Collision|SetCollisionEnabled (Variables|Default|GetBelt) "NoCollision")
      (Rendering|SetVisibility _holsterback false false)
      (Variables|Default|SetIsAttachedToPawn false)))
  (Components|StaticMesh|SetStaticMesh (Variables|Default|GetBelt) (select (Utilities|IsValid _custombeltmesh) _custombeltmesh "/Game/VR_Swords/Meshes/SM_Belt.SM_Belt"))
  (Components|StaticMesh|SetStaticMesh (Variables|Default|GetHolsterBack) (select (Utilities|IsValid _custombackmesh) _custombackmesh "/Game/VR_Swords/Meshes/SM_HolsterBack.SM_HolsterBack"))
  (if (Variables|Default|GetMakeMeshTransparent)
    (bind _returnvalue (Rendering|Material|CreateDynamicMaterialInstance "/Game/VR_Swords/Materials/M_Holster_Inst.M_Holster_Inst" "None" :!class /Script/Engine.KismetMaterialLibrary))
    (bind _output_get (Variables|Default|SetDyn_TransparentMat _returnvalue))
    (Rendering|Material|SetMaterial (Variables|Default|GetHolsterBack) 0 _output_get)
    (Rendering|Material|SetScalarParameterValue (Variables|Default|GetDyn_TransparentMat) "Opacity" (Variables|Default|GetMeshOpacity) :!class /Script/Engine.MaterialInstanceDynamic)
    (Development|SetHiddeninGame (Variables|Default|GetBelt) (Variables|Default|GetHideInGame) false)
    (Utilities|IsValid _customfixedmesh
      (:Is%20Valid
        (Components|StaticMesh|SetStaticMesh (Variables|Default|GetFixedMount) _customfixedmesh)))))