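; BP_SpectatorCam is a VR spectator camera pawn that shows a scene capture on the spectator screen.
; C toggles between the headset's cropped eye view and the render texture.
; H switches 720p and 1080p targets, while Add and Subtract adjust FOV.
; While active, Tick manually calls CaptureScene through nested FlipFlops that skip some frames to reduce capture cost.
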(event EventBeginPlay
  (bind _hires (Variables|Default|GetHiRes))
  (Variables|Default|SetIsActive false)
  (Input|EnableInput (Game|GetPlayerController 0))
  (Class|HeadMountedDisplayFunctionLibrary|SetSpectatorScreenMode "SingleEyeCroppedToFill")
  (Class|HeadMountedDisplayFunctionLibrary|SetSpectatorScreenTexture (select _hires "/Game/VR_Swords/Pawn/RT_SpectatorView1080.RT_SpectatorView1080" "/Game/VR_Swords/Pawn/RT_SpectatorView720.RT_SpectatorView720"))
  (Variables|/Script/Engine.SceneCaptureComponent2D|SetTextureTarget (Variables|Default|GetSceneCaptureComponent2D) (select _hires "/Game/VR_Swords/Pawn/RT_SpectatorView1080.RT_SpectatorView1080" "/Game/VR_Swords/Pawn/RT_SpectatorView720.RT_SpectatorView720")))

(event EventTick
  (params (DeltaSeconds :type Float%20%28single-precision%29))
  (if (Variables|Default|GetIsActive)
    (Utilities|FlowControl|FlipFlop
      (:A
        (Utilities|FlowControl|FlipFlop
          (:A
            _)
          (:B
            _)))
      (:B
        (Utilities|FlowControl|FlipFlop
          (:A
            _))))
    (Rendering|SceneCapture|CaptureScene (Variables|Default|GetSceneCaptureComponent2D) :!class /Script/Engine.SceneCaptureComponent2D)))

(event Input|KeyboardEvents|C
  (params (Key :type Key%20Structure))
  (:Pressed
    (Utilities|FlowControl|FlipFlop
      (:A
        (Class|HeadMountedDisplayFunctionLibrary|SetSpectatorScreenMode "Texture")
        (Variables|Default|SetIsActive true))
      (:B
        (Class|HeadMountedDisplayFunctionLibrary|SetSpectatorScreenMode "SingleEyeCroppedToFill")
        (Variables|Default|SetIsActive false)))))

(event Input|KeyboardEvents|Add
  (params (Key :type Key%20Structure))
  (bind _scenecapturecomponent2d (Variables|Default|GetSceneCaptureComponent2D))
  (:Pressed
    (Variables|/Script/Engine.SceneCaptureComponent2D|SetFOVAngle _scenecapturecomponent2d (- (Variables|/Script/Engine.SceneCaptureComponent2D|GetFOVAngle _scenecapturecomponent2d) 2.0))
    (Development|PrintString (Utilities|String|ToString(Float) (Variables|/Script/Engine.SceneCaptureComponent2D|GetFOVAngle _scenecapturecomponent2d)))))

(event Input|KeyboardEvents|Subtract
  (params (Key :type Key%20Structure))
  (bind _scenecapturecomponent2d (Variables|Default|GetSceneCaptureComponent2D))
  (:Pressed
    (Variables|/Script/Engine.SceneCaptureComponent2D|SetFOVAngle _scenecapturecomponent2d (+ (Variables|/Script/Engine.SceneCaptureComponent2D|GetFOVAngle _scenecapturecomponent2d) 2.0))
    (Development|PrintString (Utilities|String|ToString(Float) (Variables|/Script/Engine.SceneCaptureComponent2D|GetFOVAngle _scenecapturecomponent2d)))))

(event Input|KeyboardEvents|H
  (params (Key :type Key%20Structure))
  (:Pressed
    (bind _isa (Utilities|FlowControl|FlipFlop)
      (:A
        _)
      (:B
        _))
    (bind _output_get (Variables|Default|SetHiRes _isa))
    (Development|PrintString (select _output_get "1080p" "720p"))
    (Class|HeadMountedDisplayFunctionLibrary|SetSpectatorScreenTexture (select _output_get "/Game/VR_Swords/Pawn/RT_SpectatorView1080.RT_SpectatorView1080" "/Game/VR_Swords/Pawn/RT_SpectatorView720.RT_SpectatorView720"))
    (Variables|/Script/Engine.SceneCaptureComponent2D|SetTextureTarget (Variables|Default|GetSceneCaptureComponent2D) (select _output_get "/Game/VR_Swords/Pawn/RT_SpectatorView1080.RT_SpectatorView1080" "/Game/VR_Swords/Pawn/RT_SpectatorView720.RT_SpectatorView720"))))

(fn ConstructionScript)