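; CurrentScoreLabel is an actor that shows the current score from CharlieGameMode on its Score text.
; On BeginPlay it casts and caches the game mode.
; Every Tick it polls the score, hiding the whole actor while the score is zero and otherwise showing it and updating the text.
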(event EventBeginPlay
  (bind _ascharlie_game_mode (Utilities|Casting|CastToCharlieGameMode (Game|GetGameMode)))
  (Variables|Default|SetCharlieGameMode _ascharlie_game_mode))

(event Collision|EventActorBeginOverlap
  (params (OtherActor :type Actor%20Object%20Reference)))

(event EventTick
  (params (DeltaSeconds :type Float%20%28single-precision%29))
  (bind _charliegamemode (Variables|Default|GetCharlieGameMode))
  (bind _current_score (Default|GetCurrentScore _charliegamemode))
  (if (== _current_score 0)
    (Rendering|SetActorHiddenInGame true)
    (else
      (Rendering|SetActorHiddenInGame false)
      (Rendering|Components|TextRender|SetText (Variables|Default|GetScore) (Utilities|Text|ToText(Integer) _current_score)))))

(fn ConstructionScript)