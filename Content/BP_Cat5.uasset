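; BP_Cat5 is a cat pawn that walks toward a table and flees when hit by cheese.
; On BeginPlay it plays a slowed looping walk animation and uses AI MoveTo toward the first actor tagged "Table".
; An actor hit from a "Cheese"-tagged actor switches it to a run animation and sends it to a random "CatDespawner" actor.
; Hitting a "CatDespawner" destroys the cat.
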(event Custom|On%20Actor%20Hit
  (params (SelfActor :type Actor%20Object%20Reference) (OtherActor :type Actor%20Object%20Reference) (NormalImpulse :type Vector) (Hit :type Hit%20Result%20Structure%20%28by%20ref%29))
  (bind _skeletalmesh (Variables|Default|GetSkeletalMesh))
  (if (Actor|ActorHasTag OtherActor "Cheese")
    (bind _outactors (Actor|GetAllActorswithTag "CatDespawner"))
    (Components|Animation|PlayAnimation _skeletalmesh "/Game/Cat/Cat_Run_Anim.Cat_Run_Anim" true)
    (Components|Timeline|SetPlayRate _skeletalmesh 1.0)
    (AI|AIMoveTo self "0, 0, 0" (Utilities|Array|Get(acopy) _outactors (Math|Random|RandomInteger (Utilities|Array|Length _outactors))) 5.0 false)
    (elif (Actor|ActorHasTag OtherActor "CatDespawner")
      (Actor|DestroyActor))))

(event EventBeginPlay
  (bind _skeletalmesh (Variables|Default|GetSkeletalMesh))
  (Collision|AssignOnActorHit (delegate Custom|On%20Actor%20Hit))
  (Components|Animation|PlayAnimation _skeletalmesh "/Game/Cat/Cat_Walk_Anim.Cat_Walk_Anim" true)
  (Components|Timeline|SetPlayRate _skeletalmesh 0.5)
  (bind _outactors (Actor|GetAllActorswithTag "Table"))
  (AI|AIMoveTo self "0, 0, 0" (Utilities|Array|Get(acopy) _outactors) 5.0 false))

(event Collision|EventActorBeginOverlap
  (params (OtherActor :type Actor%20Object%20Reference)))

(event EventTick
  (params (DeltaSeconds :type Float%20%28single-precision%29)))

(fn ConstructionScript)