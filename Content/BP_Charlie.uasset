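; Cat pawn that registers with CharlieGameMode on spawn and can be fed cheese or leap onto the table.
; When hit by cheese, it reports being fed, slows, moves to eat it, then heads to a random CatDespawner and is destroyed on overlap.
; Overlapping TableBounds triggers a one-time physics impulse toward a fixed spot, then settles it there and sets GameOver, disabling feeding.
; Tick tracks speed, presumably for animation.
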(event Custom|On%20Actor%20Hit
  (params (SelfActor :type Actor%20Object%20Reference) (OtherActor :type Actor%20Object%20Reference) (NormalImpulse :type Vector) (Hit :type Hit%20Result%20Structure%20%28by%20ref%29))
  (if (not (Variables|Default|GetGameOver))
    (Utilities|IsValid OtherActor
      (:Is%20Valid
        (Development|PrintString "CatIsHit")
        (if (Actor|ActorHasTag OtherActor "Cheese")
          (bind _asbp_cheese (Utilities|Casting|CastToBP_Cheese OtherActor))
          (if (not (Variables|Default|GetIsFed))
            ;[1 1 1] Eat Cheese and wander off
            (Variables|Default|SetIsFed true)
            (Default|CatIsFed (Variables|Default|GetCharlieGameMode) self)
            (Variables|/Script/Engine.FloatingPawnMovement|SetMaxSpeed (Variables|Default|GetFloatingPawnMovement) 4e+01)
            (AI|AIMoveTo (AI|GetAIController self) "0.000000,0.000000,0.000000" _asbp_cheese 4.0 "Default" "Default" true true true
              (:then
                (Utilities|FlowControl|Delay 4.0)
                (Actor|DestroyActor _asbp_cheese)
                (bind _outactors (Actor|GetAllActorswithTag "CatDespawner"))
                (AI|AIMoveTo (AI|GetAIController self) "-545.000000,30.000000,270.000000" (Utilities|Array|Get(acopy) _outactors (Math|Random|RandomInteger (Utilities|Array|Length _outactors))) -1.0 "Default" "Default" true true)))))))))

(event Custom|OnActorBeginOverlap_Event_0
  (params (OverlappedActor :type Actor%20Object%20Reference) (OtherActor :type Actor%20Object%20Reference))
  (if (Actor|ActorHasTag OtherActor "CatDespawner")
    (Actor|DestroyActor)
    (elif (Actor|ActorHasTag OtherActor "TableBounds")
      (Utilities|FlowControl|DoOnce false
        (:Completed
          (Components|Movement|StopMovementImmediately (Variables|Default|GetFloatingPawnMovement))
          (Physics|SetSimulatePhysics (Variables|Default|GetBox) true)
          (Collision|SetCollisionEnabled (Variables|Default|GetBox) "PhysicsOnly")
          (Physics|SetEnableGravity (Variables|Default|GetBox) true)
          (Variables|Default|SetIsJumping true)
          (Physics|AddImpulse (Variables|Default|GetBox) (+ (* (- "-545.000000,20.000000,273.000000" (Transformation|GetWorldLocation (Variables|Default|GetBox))) "1.000000,1.000000,1.000000") "0.000000,0.000000,400.000000") "None" true)
          (Variables|Default|SetGameOver true)
          (Utilities|FlowControl|Delay 0.8)
          (Physics|SetSimulatePhysics (Variables|Default|GetBox) false)
          (Physics|SetEnableGravity (Variables|Default|GetBox) false)
          (Components|Movement|StopMovementImmediately (Variables|Default|GetFloatingPawnMovement))
          (Collision|SetCollisionEnabled (Variables|Default|GetBox) "NoCollision")
          (Variables|Default|SetGameOver true)
          (Variables|Default|SetIsJumping false)
          (Variables|Default|SetIsResting true)
          (Components|MoveComponentTo (Variables|Default|GetBox) "-545.000000,0.000000,273.000000" (Math|Rotator|MakeRotator 0.0 0.0 (.Yaw (Math|Rotator|BreakRotator (Transformation|GetWorldRotation (Variables|Default|GetBox))))) false false 0.2 true)
          (CallFunction|GetClosestCheese)
          (Components|MoveComponentTo 0 "-545.000000,0.000000,273.000000" "0, 0, 0" false false 0.2 true))))))

(event Custom|Start%20Moving%20Towards
  (params (TargetActor :type Actor%20Object%20Reference))
  (AI|AIMoveTo self "0, 0, 0" TargetActor 5.0 false
    (:OnSuccess
      (Development|PrintString "Movement Success"))
    (:OnFail
      (Development|PrintString "Movement Fail"))))

(event EventBeginPlay
  (bind _ascharlie_game_mode (Utilities|Casting|CastToCharlieGameMode (Game|GetGameMode)))
  (bind _output_get (Variables|Default|SetCharlieGameMode _ascharlie_game_mode))
  (Default|CatSpawned _output_get)
  (Collision|AssignOnActorHit (delegate Custom|On%20Actor%20Hit))
  (EventDispatchers|AssignOnActorBeginOverlap (delegate Custom|OnActorBeginOverlap_Event_0)))

(event Collision|EventActorBeginOverlap
  (params (OtherActor :type Actor%20Object%20Reference)))

(event EventTick
  (params (DeltaSeconds :type Float%20%28single-precision%29))
  (Variables|Default|SetSpeed (Math|Vector|VectorLength (Transformation|GetVelocity self)))
  (if (Variables|Default|GetIsFed)
    _))

(fn ConstructionScript)

(fn Meow
  (Audio|Components|Audio|Play (Variables|Default|GetMeowAudio) 0.0))

(fn EatCheeseandWanderOff
  (params (Cheese :type BP%20Cheese%20Object%20Reference)))

(fn GetClosestCheese
  (bind _outactors (Actor|GetAllActorsOfClass "/Game/BP_Cheese.BP_Cheese_C"))
  (for _array_element _outactors
    (if (< (Transformation|GetDistanceTo _array_element) (LocalVariables|GetClosestDistance))
      (LocalVariables|SetClosestCheese _array_element)
      (LocalVariables|SetClosestDistance (Transformation|GetDistanceTo _array_element))))
  (return (LocalVariables|GetClosestCheese)))