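; Cat pawn that reports spawning and being fed to CharlieGameMode, walking toward targets supplied through StartMovingTowards via AIMoveTo.
; A hit from a Cheese-tagged actor counts as feeding, speeds up its animation and sends it to a random CatDespawner, where overlap destroys it.
; Touching TableBounds once snaps it to a fixed idle pose without movement or box collision.
; Tick plays meows at random intervals while IsFed is false, though nothing here sets that flag.
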(event Custom|On%20Actor%20Hit
  (params (SelfActor :type Actor%20Object%20Reference) (OtherActor :type Actor%20Object%20Reference) (NormalImpulse :type Vector) (Hit :type Hit%20Result%20Structure%20%28by%20ref%29))
  (Development|PrintString "CatIsHit")
  (if (Actor|ActorHasTag OtherActor "Cheese")
    (Default|CatIsFed (stale EventBeginPlay _ascharlie_game_mode))
    (bind _outactors (Actor|GetAllActorswithTag "CatDespawner"))
    (Components|Timeline|SetPlayRate (Variables|Default|GetSkeletalMesh) 1.0)
    (AI|AIMoveTo self "0, 0, 0" (Utilities|Array|Get(acopy) _outactors (Math|Random|RandomInteger (Utilities|Array|Length _outactors))) 5.0 false)))

(event Custom|OnActorBeginOverlap_Event_0
  (params (OverlappedActor :type Actor%20Object%20Reference) (OtherActor :type Actor%20Object%20Reference))
  (if (Actor|ActorHasTag OtherActor "CatDespawner")
    (Actor|DestroyActor)
    (elif (Actor|ActorHasTag OtherActor "TableBounds")
      (Utilities|FlowControl|DoOnce false
        (:Completed
          (Components|Activation|Deactivate (Variables|Default|GetFloatingPawnMovement))
          (Collision|SetCollisionEnabled (Variables|Default|GetBox) "NoCollision")
          (Components|Animation|PlayAnimation (Variables|Default|GetSkeletalMesh) "/Game/Cat/Cat_Idle_Anim.Cat_Idle_Anim" true)
          (Transformation|SetActorLocationAndRotation "-545.000000,30.000000,270.000000" "0.000000,180.000000,0.000000"))))))

(event Custom|Start%20Moving%20Towards
  (params (TargetActor :type Actor%20Object%20Reference))
  (AI|AIMoveTo self "0, 0, 0" TargetActor 5.0 false
    (:OnSuccess
      (Development|PrintString "Movement Success"))
    (:OnFail
      (Development|PrintString "Movement Fail"))))

(event EventBeginPlay
  (bind _ascharlie_game_mode (Utilities|Casting|CastToCharlieGameMode (Game|GetGameMode)))
  (Default|CatSpawned _ascharlie_game_mode)
  (Collision|AssignOnActorHit (delegate Custom|On%20Actor%20Hit))
  (EventDispatchers|AssignOnActorBeginOverlap (delegate Custom|OnActorBeginOverlap_Event_0))
  (Components|Timeline|SetPlayRate (Variables|Default|GetSkeletalMesh) 0.5))

(event Collision|EventActorBeginOverlap
  (params (OtherActor :type Actor%20Object%20Reference)))

(event EventTick
  (params (DeltaSeconds :type Float%20%28single-precision%29))
  (if (not (Variables|Default|GetIsFed))
    (Utilities|FlowControl|DoOnce false :!label _label
      (:Completed
        (CallFunction|Meow)
        (Utilities|FlowControl|Delay (Math|Conversions|ToFloat(Integer) (Math|Random|RandomIntegerinRange 5 15)))
        (goto _label Reset)))))

(fn ConstructionScript)

(fn Meow
  (Audio|Components|Audio|Play (Variables|Default|GetMeowAudio) 0.0))