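; BP_Cheese is a VR sliceable cheese prop that two swords can cut and either hand can pick up piece by piece.
; Construction copies a static mesh into a procedural mesh; overlapping slice planes split listed pieces, halving mass and adding impulse, spin, haptics and sound.
; Slices notify CharlieGameMode and can start a delayed cleanup that waits until no piece is held.
; Tick releases ungripped pieces and tracks speed, which scales impact sounds and particles.
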(event Custom|EventSlice2
  (bind _sliceplane (Variables|Default|GetSlicePlane))
  (bind _procmesheslist (Variables|Default|GetProcMeshesList))
  (bind _customcapmaterial (Variables|Look|GetCustomCapMaterial))
  (bind _returnvalue (Math|Vector|GetUpVector _sliceplane))
  (bind _z (Math|Vector|BreakVector _returnvalue))
  (bind _returnvalue_2 (* _returnvalue -1.0))
  (bind _returnvalue_3 (>= _z 0.0))
  (bind _returnvalue_4 (select _returnvalue_3 _returnvalue_2 _returnvalue))
  ;[1 1 1] This event is called to slice the mesh with the second sword, if the first sword is currently slicing. This allows you to slice the same mesh simultaniously with both swords. Each component is tested and sliced if it can be sliced and is overlapping the slice plane
  (for _array_element _procmesheslist
    (for _array_element_2 (Class|PrimitiveComponent|GetOverlappingComponents _array_element)
      (if (Components|ComponentHasTag _array_element_2 "SlicePlaneComponent")
        (Utilities|Array|Add (Variables|/Script/Engine.ActorComponent|GetComponentTags _array_element) "CanSlice2"))))
  (for _array_element_3 _procmesheslist
    (if (and (Components|ComponentHasTag _array_element_3 "CanSlice2") (not (Components|ComponentHasTag _array_element_3 "Immune2")))
      (Variables|Default|SetWeightCache (/ (Variables|Default|GetWeightCache) 2.0))
      (bind _outotherhalfprocmesh (Class|KismetProceduralMeshLibrary|SliceProceduralMesh _array_element_3 (Transformation|GetWorldLocation _sliceplane) (Utilities|Select :Index (Variables|Mechanics|GetMainBodyLocation) :NewEnumerator0 (* _returnvalue_4 -1.0) :NewEnumerator1 _returnvalue_4) true "CreateNewSectionForCap" (select (Utilities|IsValid _customcapmaterial) _customcapmaterial (Rendering|Material|GetMaterial _array_element 0))))
      (Class|PrimitiveComponent|SetNotifyRigidBodyCollision _outotherhalfprocmesh true)
      (Variables|Default|SetHasBeenSliced true)
      (Class|PrimitiveComponent|SetMassOverrideinKg _outotherhalfprocmesh "None" (Variables|Default|GetWeightCache) true)
      (Utilities|Array|Add (Variables|/Script/Engine.ActorComponent|GetComponentTags _array_element_3) "Immune2")
      (Utilities|Array|Add (Variables|/Script/Engine.ActorComponent|GetComponentTags _outotherhalfprocmesh) "Immune2")
      (if (Utilities|IsValid _outotherhalfprocmesh)
        (Utilities|Array|Add (Variables|Default|GetProcMeshesList) _outotherhalfprocmesh)
        (Physics|SetSimulatePhysics _outotherhalfprocmesh true)
        (Physics|AddRadialImpulse _outotherhalfprocmesh (/ (+ (Physics|GetCenterOfMass _array_element_3 "None") (Physics|GetCenterOfMass _outotherhalfprocmesh "None")) 2.0) (Variables|Mechanics|GetSliceImpulseRadius) (Variables|Mechanics|GetSliceImpulseStrength) "RIF_Constant" true)
        (Class|PrimitiveComponent|SetPhysicsAngularVelocityinDegrees _array_element_3 (* (Math|Random|RandomUnitVector) (Variables|Default|GetSpinForce)) true "None")
        (Class|PlayerController|PlayHapticEffect (Game|GetPlayerController 0) "/Game/VR_Swords/Effects/Haptic_Slice.Haptic_Slice" (Variables|Default|GetSliceHand) 5.0 false)
        (Audio|PlaySoundatLocation (Variables|Sound|GetSliceSound) (/ (+ (Physics|GetCenterOfMass _array_element_3 "None") (Physics|GetCenterOfMass _outotherhalfprocmesh "None")) 2.0) "0, 0, 0" (Variables|Sound|GetSliceSoundVolume) 1.0 0.0 0 0 0))))
  (Utilities|FlowControl|Delay 0.1)
  (for _array_element_4 (Variables|Default|GetProcMeshesList)
    (Utilities|Array|Clear (Variables|/Script/Engine.ActorComponent|GetComponentTags _array_element_4))
    (CallFunction|EventSliced)))

(event Custom|EventSlice1
  (bind _sliceplane (Variables|Default|GetSlicePlane))
  (bind _customcapmaterial (Variables|Look|GetCustomCapMaterial))
  (bind _procmesheslist (Variables|Default|GetProcMeshesList))
  (bind _returnvalue (Math|Vector|GetUpVector _sliceplane))
  (bind _z (Math|Vector|BreakVector _returnvalue))
  (bind _returnvalue_2 (* _returnvalue -1.0))
  (bind _returnvalue_3 (>= _z 0.0))
  (bind _returnvalue_4 (select _returnvalue_3 _returnvalue_2 _returnvalue))
  ;[1 1 1] This event is called to slice the mesh. Each component is tested and sliced if it can be sliced and is overlapping the slice plane
  (for _array_element _procmesheslist
    (for _array_element_2 (Class|PrimitiveComponent|GetOverlappingComponents _array_element)
      (if (Components|ComponentHasTag _array_element_2 "SlicePlaneComponent")
        (Utilities|Array|Add (Variables|/Script/Engine.ActorComponent|GetComponentTags _array_element) "CanSlice1"))))
  (for _array_element_3 _procmesheslist
    (if (and (Components|ComponentHasTag _array_element_3 "CanSlice1") (not (Components|ComponentHasTag _array_element_3 "Immune1")))
      (Variables|Default|SetWeightCache (/ (Variables|Default|GetWeightCache) 2.0))
      (bind _outotherhalfprocmesh (Class|KismetProceduralMeshLibrary|SliceProceduralMesh _array_element_3 (Transformation|GetWorldLocation _sliceplane) (Utilities|Select :Index (Variables|Mechanics|GetMainBodyLocation) :NewEnumerator0 (* _returnvalue_4 -1.0) :NewEnumerator1 _returnvalue_4) true "CreateNewSectionForCap" (select (Utilities|IsValid _customcapmaterial) _customcapmaterial (Rendering|Material|GetMaterial _array_element 0))))
      (Class|PrimitiveComponent|SetNotifyRigidBodyCollision _outotherhalfprocmesh true)
      (Variables|Default|SetHasBeenSliced true)
      (Class|PrimitiveComponent|SetMassOverrideinKg _outotherhalfprocmesh "None" (Variables|Default|GetWeightCache) true)
      (Utilities|Array|Add (Variables|/Script/Engine.ActorComponent|GetComponentTags _array_element_3) "Immune1")
      (Utilities|Array|Add (Variables|/Script/Engine.ActorComponent|GetComponentTags _outotherhalfprocmesh) "Immune1")
      (if (Utilities|IsValid _outotherhalfprocmesh)
        (Utilities|Array|Add (Variables|Default|GetProcMeshesList) _outotherhalfprocmesh)
        (Physics|SetSimulatePhysics _outotherhalfprocmesh true)
        (Physics|AddRadialImpulse _outotherhalfprocmesh (/ (+ (Physics|GetCenterOfMass _array_element_3 "None") (Physics|GetCenterOfMass _outotherhalfprocmesh "None")) 2.0) (Variables|Mechanics|GetSliceImpulseRadius) (Variables|Mechanics|GetSliceImpulseStrength) "RIF_Constant" true)
        (Class|PrimitiveComponent|SetPhysicsAngularVelocityinDegrees _array_element_3 (* (Math|Random|RandomUnitVector) (Variables|Default|GetSpinForce)) true "None")
        (Class|PlayerController|PlayHapticEffect (Game|GetPlayerController 0) "/Game/VR_Swords/Effects/Haptic_Slice.Haptic_Slice" (Variables|Default|GetSliceHand) 5.0 false)
        (Audio|PlaySoundatLocation (Variables|Sound|GetSliceSound) (/ (+ (Physics|GetCenterOfMass _array_element_3 "None") (Physics|GetCenterOfMass _outotherhalfprocmesh "None")) 2.0) "0, 0, 0" (Variables|Sound|GetSliceSoundVolume) 1.0 0.0 0 0 0))))
  (Utilities|FlowControl|Delay 0.1)
  (for _array_element_4 (Variables|Default|GetProcMeshesList)
    (Utilities|Array|Clear (Variables|/Script/Engine.ActorComponent|GetComponentTags _array_element_4))
    (CallFunction|EventSliced)))

(event Custom|Event_ResetSliceMesh
  (bind _proceduralmesh (Variables|Default|GetProceduralMesh))
  (bind _keepmainbodystatic (Variables|Mechanics|GetKeepMainBodyStatic))
  (bind _physicsmaterialoverride (Variables|Look|GetPhysicsMaterialOverride))
  (bind _procmesheslist (Variables|Default|GetProcMeshesList))
  ;[1 1 1] Call this event to reset the procedural mesh to it's initial state
  (for _array_element _procmesheslist
    (if (!= _array_element (Variables|Default|GetProceduralMesh))
      (Components|DestroyComponent _array_element)))
  (Utilities|Array|Clear _procmesheslist)
  (Variables|Default|SetHasBeenSliced false)
  ;[1 1 1] Create Procedural mesh from static mesh and assign materials. Add Procedural Mesh to Procedural Mesh List Array(This array will contain all procedural meshes and is used to test each part when slicing and picking up)
  (Utilities|FlowControl|Delay 0.001)
  (Class|KismetProceduralMeshLibrary|CopyProceduralMeshfromStaticMeshComponent (Variables|Default|GetStaticMesh) 0 _proceduralmesh true)
  (Rendering|SetVisibility (Variables|Default|GetStaticMesh) false false)
  (Physics|SetSimulatePhysics _proceduralmesh (not _keepmainbodystatic))
  (Class|PrimitiveComponent|SetPhysMaterialOverride _proceduralmesh (select (Utilities|IsValid _physicsmaterialoverride) _physicsmaterialoverride "/Game/VR_Swords/Materials/PM_DefaultSlice.PM_DefaultSlice"))
  (if _keepmainbodystatic
    _
    (else
      (Variables|/Script/Engine.ActorComponent|SetComponentTags (Variables|Default|GetProceduralMesh) (Utilities|Array|MakeArray "Static"))))
  (Utilities|Array|Add (Variables|Default|GetProcMeshesList) (Variables|Default|GetProceduralMesh))
  (Variables|Default|SetWeightCache (Variables|Mechanics|GetWeight)))

(event Custom|Event_Sliced
  (bind _killdelay (Variables|Mechanics|GetKillDelay))
  ;[1 1 1] This event is triggered when the mesh is sliced. If Kill Delay is more than 0, the actor is destroyed after a delay equal to Kill delay. This helps with performance as multiple sliced parts can be expensive
  (bind _ascharlie_game_mode (Utilities|Casting|CastToCharlieGameMode (Game|GetGameMode)))
  (Default|CheeseSliced _ascharlie_game_mode)
  (if (> _killdelay 0.0)
    (Utilities|FlowControl|RetriggerableDelay _killdelay :!label _label)
    (if (or (Variables|Default|GetHasRightHand) (Variables|Default|GetHasLeftHand)) :!label _label_2
      (Utilities|FlowControl|Delay 1.0)
      (goto _label_2)
      (elif (Variables|Mechanics|GetAlwaysKeepMainPartAlive)
        (for _array_element (Variables|Default|GetProcMeshesList)
          (if (!= _array_element (Variables|Default|GetProceduralMesh))
            (Components|DestroyComponent _array_element)))
        (Variables|Default|SetProcMeshesList (Utilities|Array|MakeArray (Variables|Default|GetProceduralMesh)))
        (Utilities|FlowControl|DoOnce false ; enters at Reset
          (:Completed
            (goto _label)))
        (else
          (Actor|DestroyActor))))))

(event EventPickup
  (params (AttachTo :type Scene%20Component%20Object%20Reference) (Hand :type EControllerHand%20Enum :default "Left"))
  (bind _returnvalue (Components|GetOwner AttachTo))
  ;[1 1 1] This Event is triggered when the object is picked up. It works out which part is being picked up and which hand is picking it up. This uses the default PickupActorInterface from the VR template, so if your project uses a different Interface, be sure to add it to the actor and replace the pickup event with your own.
  (if (Variables|Mechanics|GetCanBePickedUp)
    (bind _asbp_motion_controller_swords (Utilities|Casting|CastToBP_MotionControllerSwords _returnvalue))
    (switch Utilities|FlowControl|Switch|SwitchonEControllerHand Hand
      (:Left
        (Variables|Default|SetLeftHandRef _asbp_motion_controller_swords)
        (for (_array_element _array_index) (Variables|Default|GetProcMeshesList)
          (for _array_element_2 (Collision|GetOverlappingActors _array_element "/Game/VR_Swords/Pawn/BP_MotionControllerSwords.BP_MotionControllerSwords_C" :!class /Script/Engine.PrimitiveComponent)
            (if (== _array_element_2 _returnvalue)
              (if (Components|ComponentHasTag _array_element "PickedUpRight")
                (Variables|Default|SetHasRightHand false))
              (Variables|/Script/Engine.ActorComponent|SetComponentTags _array_element (Utilities|Array|MakeArray "PickedUpLeft"))
              (if (== _array_index 0)
                (Variables|Mechanics|SetKeepMainBodyStatic true))
              (Physics|SetSimulatePhysics _array_element false)
              (Transformation|AttachComponentToComponent _array_element AttachTo "None" "KeepWorld" "KeepWorld" "KeepWorld" false)
              (Utilities|FlowControl|Delay 0.2)
              (Variables|Default|SetHasLeftHand true)))))
      (:Right
        (Variables|Default|SetRightHandRef _asbp_motion_controller_swords)
        (for (_array_element_3 _array_index_2) (Variables|Default|GetProcMeshesList)
          (for _array_element_4 (Collision|GetOverlappingActors _array_element_3 "/Game/VR_Swords/Pawn/BP_MotionControllerSwords.BP_MotionControllerSwords_C" :!class /Script/Engine.PrimitiveComponent)
            (if (== _array_element_4 _returnvalue)
              (if (Components|ComponentHasTag _array_element_3 "PickedUpLeft")
                (Variables|Default|SetHasLeftHand false))
              (Variables|/Script/Engine.ActorComponent|SetComponentTags _array_element_3 (Utilities|Array|MakeArray "PickedUpRight"))
              (if (== _array_index_2 0)
                (Variables|Mechanics|SetKeepMainBodyStatic true))
              (Physics|SetSimulatePhysics _array_element_3 false)
              (Transformation|AttachComponentToComponent _array_element_3 AttachTo "None" "KeepWorld" "KeepWorld" "KeepWorld" false)
              (Utilities|FlowControl|Delay 0.2)
              (Variables|Default|SetHasRightHand true))))))))

(event EventTick
  (params (DeltaSeconds :type Float%20%28single-precision%29))
  (bind _speedscene (Variables|Default|GetSpeedScene))
  (bind _returnvalue (Transformation|GetWorldLocation _speedscene))
  ;[1 1 1] Check to see if hands are gripping when a component is picked up. If the hand holding the component is not gripping, the component is dropped. This method allows picking up any of the parts that are sliced, and even picking up 2 parts of the same actor with different hands
  (Utilities|FlowControl|Sequence
    (:then_0
      (if (Variables|Default|GetHasLeftHand)
        (for _array_element (Variables|Default|GetProcMeshesList)
          (for _array_element_2 (Variables|/Script/Engine.ActorComponent|GetComponentTags _array_element)
            (if (Utilities|Name|Equal(Name) _array_element_2 "PickedUpLeft")
              (if (not (Utilities|Enum|Equal(Enum) (Variables|/Game/VR_Swords/Pawn/BP_MotionControllerSwords.BP_MotionControllerSwords_C|GetGripState (Variables|Default|GetLeftHandRef)) "NewEnumerator2"))
                (Variables|/Script/Engine.ActorComponent|SetComponentTags _array_element (Utilities|Array|MakeArray "None"))
                (Physics|SetSimulatePhysics _array_element true)
                (Transformation|DetachFromComponent _array_element "KeepRelative" "KeepRelative" "KeepRelative" true)
                (Variables|Default|SetHasLeftHand false)))))))
    (:then_1
      (if (Variables|Default|GetHasRightHand)
        (for _array_element_3 (Variables|Default|GetProcMeshesList)
          (for _array_element_4 (Variables|/Script/Engine.ActorComponent|GetComponentTags _array_element_3)
            (if (Utilities|Name|Equal(Name) _array_element_4 "PickedUpRight")
              (if (not (Utilities|Enum|Equal(Enum) (Variables|/Game/VR_Swords/Pawn/BP_MotionControllerSwords.BP_MotionControllerSwords_C|GetGripState (Variables|Default|GetRightHandRef)) "NewEnumerator2"))
                (Variables|/Script/Engine.ActorComponent|SetComponentTags _array_element_3 (Utilities|Array|MakeArray "None"))
                (Physics|SetSimulatePhysics _array_element_3 true)
                (Transformation|DetachFromComponent _array_element_3 "KeepRelative" "KeepRelative" "KeepRelative" true)
                (Variables|Default|SetHasRightHand false)))))))
    (:then_2
      ;[1 1 1] Get the speed of the object
      (bind _output_get (Variables|Default|SetObjectDeltaLocation (- _returnvalue (Variables|Default|GetLocationCache))))
      (Variables|Default|SetObjectSpeed (* (/ (Math|Vector|VectorLength _output_get) DeltaSeconds) 0.04))
      (Variables|Default|SetLocationCache _returnvalue))))

(event EventBeginPlay
  (Variables|Default|SetTags (Utilities|Array|MakeArray "Cheese"))
  (Physics|SetSimulatePhysics (Variables|Default|GetProceduralMesh) (not (Variables|Mechanics|GetKeepMainBodyStatic))))

(event Collision|EventHit
  (params (MyComp :type Primitive%20Component%20Object%20Reference) (Other :type Actor%20Object%20Reference) (OtherComp :type Primitive%20Component%20Object%20Reference) (bSelfMoved :type Boolean) (HitLocation :type Vector :default "0, 0, 0") (HitNormal :type Vector :default "0, 0, 0") (NormalImpulse :type Vector :default "0, 0, 0") (Hit :type Hit%20Result%20Structure%20%28by%20ref%29))
  (bind _objectspeed (Variables|Default|GetObjectSpeed))
  (bind _hitparticleeffect (Variables|Look|GetHitParticleEffect))
  (bind _hitsoundhard (Variables|Sound|GetHitSoundHard))
  (bind _hitsoundsoft (Variables|Sound|GetHitSoundSoft))
  (bind _returnvalue (< _objectspeed 12.0))
  (bind _returnvalue_2 (select _returnvalue _hitsoundsoft _hitsoundhard))
  ;[1 1 1] Play Sound and particle effects when the object hits other objects
  (Utilities|FlowControl|DoOnce false :!label _label
    (:Completed
      (Utilities|IsValid _returnvalue_2
        (:Is%20Valid
          (Audio|PlaySoundatLocation _returnvalue_2 HitLocation "0, 0, 0" (Math|Float|MapRangeClamped _objectspeed 4.0 2e+01 0.0 1.0) 0.75 0.0 0 0 0))
        (:Is%20Not%20Valid
          _))
      (if (> _objectspeed 8.0)
        (Utilities|IsValid _hitparticleeffect
          (:Is%20Valid
            (Effects|SpawnEmitteratLocation _hitparticleeffect HitLocation (Math|Rotator|MakeRotfromZ HitNormal) (Math|Conversions|ToVector(Float) (Math|Float|MapRangeClamped _objectspeed 7.0 2e+01 0.04 0.2))))
          (:Is%20Not%20Valid
            _)))
      (Utilities|FlowControl|Delay 0.3)
      (goto _label Reset))))

(event Collision|EventActorBeginOverlap
  (params (OtherActor :type Actor%20Object%20Reference))
  ;[1 1 1] Check to see if overlapping actor is a sword and if it's slice plane is active. This also drops picked up pieces when the mesh is sliced, as slicing a mesh while holding it can cause issues otherwise
  (if (Actor|ActorHasTag OtherActor "Left")
    (Variables|Default|SetSliceHand "Left")
    (elif (Actor|ActorHasTag OtherActor "Right")
      (Variables|Default|SetSliceHand "Right")))
  (if (== OtherActor (Variables|Default|GetSword1Ref))
    _
    (elif (Utilities|IsValid (Variables|Default|GetSword1Ref))
      (Variables|Default|SetSword2Ref OtherActor)
      (else
        (Variables|Default|SetSword1Ref OtherActor))))
  (for _array_element (Actor|GetComponentsbyTag OtherActor "/Script/Engine.StaticMeshComponent" "SlicePlaneComponent")
    (Variables|Default|SetSlicePlane _array_element)
    (if (== OtherActor (Variables|Default|GetSword1Ref))
      (CallFunction|EventSlice1)
      (else
        (CallFunction|EventSlice2)))
    (if (or (Variables|Default|GetHasRightHand) (Variables|Default|GetHasLeftHand))
      (for (_array_element_2 _array_index) (Variables|Default|GetProcMeshesList)
        (if (not (and (not (Variables|Mechanics|GetKeepMainBodyStatic)) (== _array_index 0)))
          (Physics|SetSimulatePhysics _array_element_2 true)
          (Transformation|DetachFromComponent _array_element_2 "KeepRelative" "KeepRelative" "KeepRelative" true)))
      (Variables|Default|SetHasRightHand false)
      (Variables|Default|SetHasLeftHand false)
      (else
        (Utilities|FlowControl|RetriggerableDelay 0.5)
        (Variables|Default|SetSword1Ref 0)
        (Variables|Default|SetSword2Ref 0)))))

(fn ConstructionScript
  (bind _custommainmaterial (Variables|Look|GetCustomMainMaterial))
  (bind _proceduralmesh (Variables|Default|GetProceduralMesh))
  (bind _staticmesh (Variables|Default|GetStaticMesh))
  (bind _keepmainbodystatic (Variables|Mechanics|GetKeepMainBodyStatic))
  (bind _physicsmaterialoverride (Variables|Look|GetPhysicsMaterialOverride))
  ;[1 1 1] Assign Mesh and materials
  (Variables|Default|SetTags (Utilities|Array|MakeArray (select (Variables|Mechanics|GetCanStickWithThrownSwords) "CanStick" "")))
  (Class|PrimitiveComponent|SetMassOverrideinKg (Variables|Default|GetProceduralMesh) "None" (Variables|Mechanics|GetWeight) true)
  (Components|StaticMesh|SetStaticMesh _staticmesh (Variables|Look|GetMesh))
  (Rendering|Material|SetMaterial _staticmesh 0 (select (Utilities|IsValid _custommainmaterial) _custommainmaterial (Rendering|Material|GetMaterial _staticmesh 0)))
  ;[1 1 1] Create Procedural mesh from static mesh and assign materials. Add Procedural Mesh to Procedural Mesh List Array(This array will contain all procedural meshes and is used to test each part when slicing and picking up)
  (Class|KismetProceduralMeshLibrary|CopyProceduralMeshfromStaticMeshComponent (Variables|Default|GetStaticMesh) 0 _proceduralmesh true)
  (Rendering|SetVisibility (Variables|Default|GetStaticMesh) false false)
  (Physics|SetSimulatePhysics _proceduralmesh (not _keepmainbodystatic))
  (Class|PrimitiveComponent|SetPhysMaterialOverride _proceduralmesh (select (Utilities|IsValid _physicsmaterialoverride) _physicsmaterialoverride "/Game/VR_Swords/Materials/PM_DefaultSlice.PM_DefaultSlice"))
  (if _keepmainbodystatic
    _
    (else
      (Variables|/Script/Engine.ActorComponent|SetComponentTags (Variables|Default|GetProceduralMesh) (Utilities|Array|MakeArray "Static"))))
  (Utilities|Array|Add (Variables|Default|GetProcMeshesList) (Variables|Default|GetProceduralMesh))
  (Variables|Default|SetWeightCache (Variables|Mechanics|GetWeight)))